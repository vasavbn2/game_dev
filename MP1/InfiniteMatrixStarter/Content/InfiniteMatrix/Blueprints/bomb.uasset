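; Bomb hazard actor that explodes when a player or rocket interacts with its Box trigger.
; Player overlap start subtracts clamped health, plays explosion sound and camera shake, then destroys the bomb.
; Rocket overlap end also destroys the bomb with sound and shake, though that shake leaves its epicenter unset.
; Player overlap end adds one point to that player's Score.
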(event OnComponentBeginOverlap(Box)
  (params (OverlappedComponent :type Primitive%20Component%20Object%20Reference) (OtherActor :type Actor%20Object%20Reference) (OtherComp :type Primitive%20Component%20Object%20Reference) (OtherBodyIndex :type Integer) (bFromSweep :type Boolean) (SweepResult :type Hit%20Result%20Structure%20%28by%20ref%29))
  (bind _asbp_player (Utilities|Casting|CastToBP_Player OtherActor))
  (Variables|/Game/InfiniteMatrix/Blueprints/BP_Player.BP_Player_C|SetHealth _asbp_player (Math|Float|Clamp(Float) (- (Variables|/Game/InfiniteMatrix/Blueprints/BP_Player.BP_Player_C|GetHealth _asbp_player) 2e+01) 0.0 1e+02))
  (Audio|PlaySoundatLocation "/Game/InfiniteMatrix/sounds/mixkit-arcade-game-explosion-2759.mixkit-arcade-game-explosion-2759" (Transformation|GetWorldLocation (Variables|Default|GetBox)) "0, 0, 0" 1.0 1.0 0.0 0 0 0 0)
  (Camera|PlayWorldCameraShake "/Game/InfiniteMatrix/Blueprints/camera_shake.camera_shake_C" (Transformation|GetActorLocation _asbp_player) 0.0 5e+02)
  (Actor|DestroyActor))

(event OnComponentEndOverlap(Box)
  (params (OverlappedComponent :type Primitive%20Component%20Object%20Reference) (OtherActor :type Actor%20Object%20Reference) (OtherComp :type Primitive%20Component%20Object%20Reference) (OtherBodyIndex :type Integer))
  (Utilities|FlowControl|Sequence
    (:then_0
      (Utilities|Casting|CastTorocket OtherActor)
      (Actor|DestroyActor)
      (Audio|PlaySoundatLocation "/Game/InfiniteMatrix/sounds/mixkit-arcade-game-explosion-2759.mixkit-arcade-game-explosion-2759" (Transformation|GetWorldLocation (Variables|Default|GetBox)) "0, 0, 0" 1.0 1.0 0.0 0 0 0 0)
      (Camera|PlayWorldCameraShake "/Game/InfiniteMatrix/Blueprints/camera_shake.camera_shake_C" "0, 0, 0" 0.0 5e+02)
      (Actor|DestroyActor))
    (:then_1
      (bind _asbp_player (Utilities|Casting|CastToBP_Player OtherActor))
      (Variables|/Game/InfiniteMatrix/Blueprints/BP_Player.BP_Player_C|Setscore _asbp_player (+ (Variables|/Game/InfiniteMatrix/Blueprints/BP_Player.BP_Player_C|Getscore _asbp_player) 1)))))

(event EventBeginPlay)

(event Collision|EventActorBeginOverlap
  (params (OtherActor :type Actor%20Object%20Reference)))

(event EventTick
  (params (DeltaSeconds :type Float%20%28single-precision%29)))

(fn ConstructionScript)